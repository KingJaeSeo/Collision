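; BP_MoveUpDown is an actor whose Cube component bounces up and down along its relative Z axis while IsPlay is true.
; Tick moves it a fixed step each frame, unscaled by delta time, flipping IsMoveRight (which actually means upward) at EndPoint and below zero.
; The Play function sets IsPlay to start or stop the motion.
; The F key only prints press and release messages.
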(event `self.ReceiveTick`
  (params (DeltaSeconds :type "Float (single-precision)"))
  (bind _cube (`self.Cube`))
  (bind (_relativelocation_x _relativelocation_y _relativelocation_z) (`KismetMathLibrary.BreakVector` (`SceneComponent.RelativeLocation` _cube)))
  (bind (_relativelocation_x_2 _relativelocation_y_2 _relativelocation_z_2) (`KismetMathLibrary.BreakVector` (`SceneComponent.RelativeLocation` _cube)))
  (if (`self.IsPlay`)
    (if (`self.IsMoveRight`)
      (`SceneComponent.K2_AddRelativeLocation` _cube (0.0 0.0 5.0) false false)
      (if (>= _relativelocation_z_2 (`self.EndPoint`))
        (set `self.IsMoveRight` false))
      (else
        (`SceneComponent.K2_AddRelativeLocation` (`self.Cube`) (0.0 0.0 -5.0) false false)
        (if (< _relativelocation_z 0.0)
          (set `self.IsMoveRight` true))))))

(event `Key|F`
  (params (Key :type "Key Structure"))
  (:`Pressed`
    (`KismetSystemLibrary.PrintString` "F key pressed"))
  (:`Released`
    (`KismetSystemLibrary.PrintString` "F key released")))

(fn `Play`
  (params (IsPlay :type Boolean))
  (set `self.IsPlay` IsPlay))

(fn `UserConstructionScript`)